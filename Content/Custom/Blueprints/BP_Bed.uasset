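; BP_Bed is a bed actor that detects when the character is close enough to rest.
; Its Box overlap events react only to the Character's capsule, setting IsBedNear on the character and toggling the bed's input for player controller 0.
; Entering adds a new X_Rest widget to the viewport and leaving removes it.
; The bed's graph holds no input handling or rest logic.
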(event `self.Box.OnComponentBeginOverlap`
  (params (OverlappedComponent :type "PrimitiveComponent Object Reference") (OtherActor :type "Actor Object Reference") (OtherComp :type "PrimitiveComponent Object Reference") (OtherBodyIndex :type Integer) (bFromSweep :type Boolean) (SweepResult :type "HitResult Structure (by ref)"))
  (bind _character (`self.Character`))
  (if (== (`Character.CapsuleComponent` _character) OtherComp)
    (`self.EnableInput` (`GameplayStatics.GetPlayerController` 0))
    (set `/Game/Custom/Blueprints/FirstPersonCharacter_2.is_bed_near?` true _character)
    (bind _returnvalue (`|CreateWidget` "/Game/Custom/Widget/X_Rest.X_Rest_C"))
    (`UserWidget.AddToViewport` _returnvalue 0)))

(event `self.Box.OnComponentEndOverlap`
  (params (OverlappedComponent :type "PrimitiveComponent Object Reference") (OtherActor :type "Actor Object Reference") (OtherComp :type "PrimitiveComponent Object Reference") (OtherBodyIndex :type Integer))
  (bind _character (`self.Character`))
  (if (== (`Character.CapsuleComponent` _character) OtherComp)
    (`self.DisableInput` (`GameplayStatics.GetPlayerController` 0))
    (set `/Game/Custom/Blueprints/FirstPersonCharacter_2.is_bed_near?` false _character)
    (`Widget.RemoveFromParent` (stale `self.Box.OnComponentBeginOverlap` _returnvalue))))

(fn `UserConstructionScript`)