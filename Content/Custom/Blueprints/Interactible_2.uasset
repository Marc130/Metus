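; Pickup actor for food, medicine or firematches, with its mesh set from TypeChoise in the construction script.
; Box overlap with Character enables input and shows prompts to pick up, or use food and medicine in place.
; Pickups update Character stats and UI, with a small food poisoning chance and one-item food and medicine limits warned under a GameInstance cooldown.
; Taken items teleport below the world instead of being destroyed, and Spawn restores them.
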(event `InputAction|Use in place`
  (params (Key :type "Key Structure"))
  (bind _character (`self.Character`))
  (bind _character_2 (`self.Character`))
  (bind _character_3 (`self.Character`))
  ;[1 1 1] Y interaction
  (:`Pressed`
    (if (`self.In_Range`)
      (switch `/Game/Custom/Blueprints/ENUM_interactible` (cast `/Game/Custom/Blueprints/ENUM_interactible` (`self.Type Choise`))
        (:`NewEnumerator1`
          (bind _output_get (set `self.Poisoned` (> (`KismetMathLibrary.RandomInteger` 100) 95)))
          (if _output_get
            (set `/Game/Custom/Blueprints/FirstPersonCharacter_2.Health` (+ (`/Game/Custom/Blueprints/FirstPersonCharacter_2.Health` _character_3) -0.2) _character_3))
          (set `/Game/Custom/Blueprints/FirstPersonCharacter_2.Hunger` (+ (`/Game/Custom/Blueprints/FirstPersonCharacter_2.Hunger` _character) 0.2) _character)
          ;[1 1 1] Poisoned Food
          (if (`self.Poisoned`) :!label _label
            (set `/Game/Custom/Blueprints/FirstPersonCharacter_2.Poisoned_Character` true (`self.Character`))
            (set `self.Poisoned` false)))
        (:`NewEnumerator2`
          (set `/Game/Custom/Blueprints/FirstPersonCharacter_2.Health` (+ (`/Game/Custom/Blueprints/FirstPersonCharacter_2.Health` _character_2) 0.2) _character_2)))
      (`self.K2_SetActorLocation` (0.0 0.0 -1000.0) :!label _label_2)
      (set `self.Exists` false))))

(event `InputAction|Interact`
  (params (Key :type "Key Structure"))
  (bind _character (`self.Character`))
  (bind _ascooldown (cast `/Game/Custom/Blueprints/Cooldown` (`GameplayStatics.GetGameInstance`) :!pure true))
  (bind _ui (`/Game/Custom/Blueprints/FirstPersonCharacter_2.UI` _character))
  (bind _food (`/Game/Custom/Blueprints/FirstPersonCharacter_2.Food` _character))
  (bind _cooldown (`/Game/Custom/Blueprints/Cooldown.Cooldown` _ascooldown))
  (:`Pressed`
    (if (`self.In_Range`)
      (switch `/Game/Custom/Blueprints/ENUM_interactible` (cast `/Game/Custom/Blueprints/ENUM_interactible` (`self.Type Choise`))
        (:`NewEnumerator0`
          ;[1 1 1] +Firematch
          (set `/Game/Custom/Blueprints/FirstPersonCharacter_2.Firematch` (+ (`/Game/Custom/Blueprints/FirstPersonCharacter_2.Firematch` _character) 1) _character)
          ;[1 1 1] UI Update
          (`EditableTextBox.SetHintText` (`/Game/Custom/Widget/UI_StatusBars.Firematch` _ui) (`KismetTextLibrary.Conv_IntToText` 1))
          (goto _label_2))
        (:`NewEnumerator1`
          (if (>= (`/Game/Custom/Blueprints/FirstPersonCharacter_2.Food` _character) 1)
            ;[1 1 1] Too much food
            (if (not _cooldown)
              (bind _returnvalue (`|CreateWidget` "/Game/Custom/Widget/Too_Much_Food.Too_Much_Food_C"))
              (`UserWidget.AddToViewport` _returnvalue 0)
              (set `/Game/Custom/Blueprints/Cooldown.Cooldown` true _ascooldown)
              (`KismetSystemLibrary.Delay` 1.2)
              (set `/Game/Custom/Blueprints/Cooldown.Cooldown` false _ascooldown)
              (`Widget.RemoveFromParent` _returnvalue))
            (else
              (bind _output_get (set `self.Poisoned` (> (`KismetMathLibrary.RandomInteger` 100) 95)))
              ;[1 1 1] + Food
              (if _output_get
                ;[1 1 1] Poisoned Food
                (set `/Game/Custom/Blueprints/FirstPersonCharacter_2.Food` (+ _food 1) _character)
                (goto _label)
                (else
                  (set `/Game/Custom/Blueprints/FirstPersonCharacter_2.Food` (+ _food 1) _character)
                  (`EditableTextBox.SetHintText` (`/Game/Custom/Widget/UI_StatusBars.Food` _ui) (`KismetTextLibrary.Conv_IntToText` 1))
                  (goto _label_2))))))
        (:`NewEnumerator2`
          ;[1 1 1] + Medicine
          (if (>= (`/Game/Custom/Blueprints/FirstPersonCharacter_2.Medicines` _character) 1)
            ;[1 1 1] Too much medkits
            (if (not _cooldown)
              (bind _returnvalue_2 (`|CreateWidget` "/Game/Custom/Widget/Too_Much_Medikits.Too_Much_Medikits_C"))
              (`UserWidget.AddToViewport` _returnvalue_2 0)
              (set `/Game/Custom/Blueprints/Cooldown.Cooldown` true _ascooldown)
              (`KismetSystemLibrary.Delay` 1.2)
              (set `/Game/Custom/Blueprints/Cooldown.Cooldown` false _ascooldown)
              (`Widget.RemoveFromParent` _returnvalue_2))
            (else
              (set `/Game/Custom/Blueprints/FirstPersonCharacter_2.Medicines` (+ (`/Game/Custom/Blueprints/FirstPersonCharacter_2.Medicines` _character) 1) _character)
              (`EditableTextBox.SetHintText` (`/Game/Custom/Widget/UI_StatusBars.Medicine` _ui) (`KismetTextLibrary.Conv_IntToText` 1))
              (goto _label_2))))))))

(event `self.Box.OnComponentBeginOverlap`
  (params (OverlappedComponent :type "PrimitiveComponent Object Reference") (OtherActor :type "Actor Object Reference") (OtherComp :type "PrimitiveComponent Object Reference") (OtherBodyIndex :type Integer) (bFromSweep :type Boolean) (SweepResult :type "HitResult Structure (by ref)"))
  ;[1 1 1] UI Prompt Spawn
  (if (== (`Character.CapsuleComponent` (`self.Character`)) OtherComp)
    (set `self.In_Range` true)
    (`self.EnableInput` (`GameplayStatics.GetPlayerController` 0))
    (bind _returnvalue (`|CreateWidget` "/Game/Custom/Widget/X_Pickup.X_Pickup_C"))
    (`UserWidget.AddToViewport` _returnvalue 0)
    (switch `/Game/Custom/Blueprints/ENUM_interactible` (cast `/Game/Custom/Blueprints/ENUM_interactible` (`self.Type Choise`))
      (:`NewEnumerator1`
        (bind _returnvalue_2 (`|CreateWidget` "/Game/Custom/Widget/Y_Eat.Y_Eat_C"))
        (`UserWidget.AddToViewport` _returnvalue_2 0))
      (:`NewEnumerator2`
        (bind _returnvalue_3 (`|CreateWidget` "/Game/Custom/Widget/Y_UseMedicine.Y_UseMedicine_C"))
        (`UserWidget.AddToViewport` _returnvalue_3 0)))))

(event `self.Box.OnComponentEndOverlap`
  (params (OverlappedComponent :type "PrimitiveComponent Object Reference") (OtherActor :type "Actor Object Reference") (OtherComp :type "PrimitiveComponent Object Reference") (OtherBodyIndex :type Integer))
  ;[1 1 1] UI Prompt Spawn
  (if (== (`Character.CapsuleComponent` (`self.Character`)) OtherComp)
    (set `self.In_Range` false)
    (`self.DisableInput` (`GameplayStatics.GetPlayerController` 0))
    (`Widget.RemoveFromParent` (stale `self.Box.OnComponentBeginOverlap` _returnvalue))
    (switch `/Game/Custom/Blueprints/ENUM_interactible` (cast `/Game/Custom/Blueprints/ENUM_interactible` (`self.Type Choise`))
      (:`NewEnumerator1`
        (`Widget.RemoveFromParent` (stale `self.Box.OnComponentBeginOverlap` _returnvalue_2)))
      (:`NewEnumerator2`
        (`Widget.RemoveFromParent` (stale `self.Box.OnComponentBeginOverlap` _returnvalue_3))))))

(event `Spawn`
  (`self.K2_SetActorLocation` (`self.Location`))
  (set `self.Exists` true))

(fn `UserConstructionScript`
  (locals (`Mesh Array` :type "Array of StaticMesh Object Reference"))
  (`StaticMeshComponent.SetStaticMesh` (`self.StaticMesh`) (`|GetArrayItem` (`local.Mesh Array`) (`KismetMathLibrary.Conv_ByteToInt` (`self.Type Choise`)))))